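; RoundManager runs battle rounds and registers itself with the GameManager game instance on BeginPlay.
; StartRound increments the round and refills the AI party with random picks from the DataManager master list, up to MonsterLimit.
; EndRound reports whether that party is wiped out, and separate handlers print victory or defeat.
; Victory calls GiveRandomItems, whose inverted-looking cap check breaks unless ItemsGranted already equals the random cap.
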(event EventBeginPlay
  (CallFunction|SystemInit))

(event Collision|EventActorBeginOverlap
  (params (OtherActor :type Actor%20Object%20Reference)))

(event EventTick
  (params (DeltaSeconds :type Float%20%28single-precision%29)))

(fn ConstructionScript)

(fn SystemInit
  (bind _asgame_manager (Utilities|Casting|CastToGameManager (Game|GetGameInstance)))
  (Default|SetRoundManager _asgame_manager self))

(fn SelectRoundMonsters
  (bind _datamanager (Variables|Default|GetDataManager))
  (bind _aiparty (Variables|Default|GetAIParty))
  (bind _monsterdatamasterlist (Variables|/Game/Blueprints/DataManager.DataManager_C|GetMonsterDataMasterList _datamanager))
  (Utilities|Array|Clear (Variables|/Game/Blueprints/PartySystem.PartySystem_C|GetMonsterDataArray _aiparty))
  (for _index (range 0 (- (Variables|Default|GetMonsterLimit) 1))
    (Utilities|Array|Add (Variables|/Game/Blueprints/PartySystem.PartySystem_C|GetMonsterDataArray _aiparty) (Utilities|Array|Get(acopy) _monsterdatamasterlist (Math|Random|RandomIntegerinRange 0 (- (Utilities|Array|Length _monsterdatamasterlist) 1))))))

(fn EndRound
  (if (not (Variables|/Game/Blueprints/PartySystem.PartySystem_C|GetAnyMonsterAlive (Variables|Default|GetAIParty)))
    (return true)
    (else
      (return false))))

(fn StartRound
  (Variables|Default|SetcurrentRound (+ (Variables|Default|GetcurrentRound) 1))
  (Development|PrintString "Starting Round" true true "(R=0.000000,G=0.660000,B=1.000000,A=1.000000)" 5.0)
  (CallFunction|SelectRoundMonsters))

(fn HandlePlayerVictory
  (Development|PrintString "Enemy Was Defeated1" true true "(R=1.000000,G=1.000000,B=1.000000,A=1.000000)" 1e+01)
  (CallFunction|GiveRandomItems))

(fn HandlePlayerLoss
  (Development|PrintString "You Have Been Defeated" true true "(R=1.000000,G=0.963542,B=0.998751,A=1.000000)" 1e+01))

(fn GiveRandomItems
  (bind _inventorymanager (Variables|Default|GetinventoryManager))
  (bind _inventoryitem (Variables|/Game/Blueprints/ItemData/InventoryManager.InventoryManager_C|GetInventoryItem _inventorymanager))
  (LocalVariables|SetrandomItemCap (Math|Random|RandomIntegerinRange 1 3))
  (Utilities|Array|ForEachLoopwithBreak _inventoryitem :!label _label
    (:LoopBody
      (if (== (LocalVariables|GetitemsGranted) (LocalVariables|GetrandomItemCap))
        (Default|AddItem _inventorymanager (Utilities|Array|Get(acopy) _inventoryitem (Math|Random|RandomIntegerinRange 0 (- (Utilities|Array|Length _inventoryitem) 1))) 1)
        (LocalVariables|SetitemsGranted (+ (LocalVariables|GetitemsGranted) 1))
        (else
          (goto _label Break))))))
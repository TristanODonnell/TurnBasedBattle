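; Battle-system Blueprint meant to calculate the effects of a monster's move on a defending monster.
; CalculateMoveEffects loops over the move's categories, sending Physical and Special to handlers that compute attack times move damage over the matching defence, truncated.
; It is unfinished: results never reach a return, and type and accuracy inputs go unused.
; Status, block and stat-change handlers are empty, unconnected stubs.
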(event EventBeginPlay)

(event Collision|EventActorBeginOverlap
  (params (OtherActor :type Actor%20Object%20Reference)))

(event EventTick
  (params (DeltaSeconds :type Float%20%28single-precision%29)))

(fn ConstructionScript)

(fn CalculateMoveEffects
  (params (AttackingMonAttack :type Float%20%28double-precision%29) (AttackingMonSpeAttack :type Float%20%28double-precision%29) (AttackingMonType :type Array%20of%20EMonsterType%20Enums :default "NewEnumerator0") (MoveCategory :type Array%20of%20EMoveCategory%20Enums :default "NewEnumerator0") (MoveAccuracy :type Float%20%28double-precision%29) (MoveType :type EMonsterType%20Enum :default "NewEnumerator0") (MoveDamage :type Float%20%28double-precision%29) (DefendingMonDefence :type Float%20%28double-precision%29) (DefendingMonSpeDefence :type Float%20%28double-precision%29) (DefendingMonType :type Array%20of%20EMonsterType%20Enums :default "NewEnumerator0"))
  (LocalVariables|SetAttack AttackingMonAttack)
  (LocalVariables|SetSpecialAttack AttackingMonSpeAttack)
  (LocalVariables|SetDefence DefendingMonDefence)
  (LocalVariables|SetSpecialDefence DefendingMonSpeDefence)
  (LocalVariables|SetMoveDamageval MoveDamage)
  (for _array_element MoveCategory
    (switch Utilities|FlowControl|Switch|SwitchonEMoveCategory _array_element
      (:NewEnumerator0
        (bind _calculateddamage (CallFunction|HandlePhysicalMove (LocalVariables|GetAttack) (LocalVariables|GetDefence) (LocalVariables|GetMoveDamageval))))
      (:NewEnumerator1
        (bind _calculateddamage_2 (CallFunction|HandleSpecialMove (LocalVariables|GetSpecialAttack) (LocalVariables|GetSpecialDefence) (LocalVariables|GetMoveDamageval)))))))

(fn HandlePhysicalMove
  (params (MonsterAttack :type Float%20%28double-precision%29) (MonsterDefence :type Float%20%28double-precision%29) (MoveDamage :type Float%20%28double-precision%29))
  (return (Math|Float|Truncate (/ (* MonsterAttack MoveDamage) MonsterDefence))))

(fn HandleSpecialMove
  (params (MonsterSpecialAttack :type Float%20%28double-precision%29) (MonsterSpecialDefence :type Float%20%28double-precision%29) (MoveDamage :type Float%20%28double-precision%29))
  (return (Math|Float|Truncate (/ (* MonsterSpecialAttack MoveDamage) MonsterSpecialDefence))))

(fn HandleBlockMove)

(fn HandleStatChangeMove)

(fn HandleStatusMove)
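; Battle system Blueprint for turn-based monster fights between a player and an AI party.
; On BeginPlay it registers with GameManager, sets up parties, starts RoundManager and binds the move selector UI.
; Each selection sets and dispatches player and AISelector actions, guarded by a turn-in-progress flag.
; Work in progress: AI slot assignment, speed/block ordering, damage resolution and end-turn reset are disconnected; item and swap logic are unfinished.
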(event Custom|handleButtonSelected
  (bind _ai_monster (Variables|Default|GetAi%20Monster))
  ;[0.15 0.15 0.15 0.5] Input Space starts event of turn phases in order
  (if (not (Variables|Default|GetisTurnInProgress))
    (Variables|Default|SetisTurnInProgress true)
    ;;[0.15 0.15 0.15 0.5] Player
    (CallFunction|SetCurrentAction (Variables|Default|Getplayer%20Monster))
    (CallFunction|CurrentActionSwitch (Variables|Default|Getplayer%20Monster))
    ;;[0.15 0.15 0.15 0.5] AI DECISION FOR TURN
    (Default|EvaluateTurnDecision (Variables|Default|GetAISelector%20))
    (CallFunction|SetCurrentAction _ai_monster)
    (CallFunction|CurrentActionSwitch _ai_monster)
    ;[1 0 0.2023 0.5] NEED TO IMPLEMENT CURRENT ACTION INTO DECISION
    (CallFunction|MoveOrderPhase)
    (else
      (Development|PrintString "STOP TURN IS IN PROGRESS"))))

(event EventBeginPlay
  (bind _player_monster (Variables|Default|Getplayer%20Monster))
  (bind _ai_monster (Variables|Default|GetAi%20Monster))
  (bind _party (Variables|/Game/Blueprints/MonsterGameSlots/BP_Monster.BP_Monster_C|GetParty _player_monster))
  (bind _party_2 (Variables|/Game/Blueprints/MonsterGameSlots/BP_Monster.BP_Monster_C|GetParty _ai_monster))
  (CallFunction|SystemInit)
  ;[0.15 0.15 0.15 0.5] Game Manager + UI Input Move Selector Setup
  (Development|PrintString "Trying to load move")
  (Utilities|FlowControl|Delay 2.0)
  (bind _asgame_manager (Utilities|Casting|CastToGameManager (Game|GetGameInstance)))
  (bind _output_get (Variables|Default|SetMove%20selecter (Variables|/Game/Blueprints/UI/UIManager.UIManager_C|GetMoveSelectorUI (Variables|/Game/Blueprints/GameManager.GameManager_C|GetUIManager _asgame_manager))))
  (Variables|Default|SetGameSlotUI (Variables|/Game/Blueprints/UI/UIManager.UIManager_C|GetAISlotUI (Variables|/Game/Blueprints/GameManager.GameManager_C|GetUIManager _asgame_manager)))
  ;[0.15 0.15 0.15 0.5] Slot Setup(see functions)
  (CallFunction|SetSlots)
  (CallFunction|SetSlotsArray)
  ;[0.15 0.15 0.15 0.5] Player Party Init
  (Default|SetMonsterInstArray _party) ; Add the data array to the instance array
  (Default|StatSetup _player_monster _party) ; Set Slot Info for Player
  ;[0.15 0.15 0.15 0.5] Start Round by Selecting AI Party
  (Default|StartRound (Variables|Default|GetRoundManager))
  ;[0.15 0.15 0.15 0.5] AI Party Selection + Init
  (Default|SetMonsterInstArray _party_2) ; Add the data array to the instance array
  (Default|StatSetup _ai_monster _party_2) ; Set Slot Info for AI
  (EventDispatchers|BindEventtoOnButtonSelected _output_get (delegate Custom|handleButtonSelected)) ; Assigning event listener
)

(fn ConstructionScript)

(fn SystemInit
  (bind _asgame_manager (Utilities|Casting|CastToGameManager (Game|GetGameInstance)))
  (Default|SetBattleSystem _asgame_manager self))

(fn SetSlots
  ;[0.15 0.15 0.15 0.5] Player Slot Setup
  (bind _asbp_monster_child_player (Utilities|Casting|CastToBP_Monster_Child_Player (Variables|/Script/Engine.ChildActorComponent|GetChildActor (Variables|Default|GetPlayerSlot)))
    (:then
      (Variables|Default|Setplayer%20Monster _asbp_monster_child_player))
    (:CastFailed
      (Development|PrintString "Cast FAILED " true true "(R=1.000000,G=0.000000,B=0.142274,A=1.000000)"))))

(fn SetSlotsArray
  (Variables|Default|SetMonsterSlots (Utilities|Array|MakeArray (Variables|Default|Getplayer%20Monster) (Variables|Default|GetAi%20Monster))))

(fn StartTurn
  (CallFunction|MoveOrderPhase))

(fn MoveOrderPhase
  (for _array_element (Variables|Default|GetMonsterSlots)
    (if (Utilities|Enum|Equal(Enum) (Variables|/Game/Blueprints/MonsterGameSlots/BP_Monster.BP_Monster_C|GetcurrentAction _array_element) "NewEnumerator0")
      _)))

(fn AttackPhase)

(fn HandleDeath
  (params (Slot :type BP%20Monster%20Object%20Reference))
  (|SetBy-RefVar (.isDead (Utilities|Struct|BreakMonsterInstance (Variables|/Game/Blueprints/PartySystem.PartySystem_C|GetcurrentMonsterInst (Variables|/Game/Blueprints/MonsterGameSlots/BP_Monster.BP_Monster_C|GetParty Slot)))) true))

(fn EndTurnPhase
  (Variables|Default|SetisTurnInProgress false))

(fn CheckPartyStatus
  (params (Game%20Slot :type BP%20Monster%20Object%20Reference))
  (bind _party (Variables|/Game/Blueprints/MonsterGameSlots/BP_Monster.BP_Monster_C|GetParty Game%20Slot))
  (bind _array_element (Utilities|Array|ForEachLoopwithBreak (Variables|/Game/Blueprints/PartySystem.PartySystem_C|GetMonsterInstanceArray _party) :!label _label)
    (:LoopBody
      (if (not (.isDead (Utilities|Struct|BreakMonsterInstance _array_element)))
        (Variables|/Game/Blueprints/PartySystem.PartySystem_C|SetAnyMonsterAlive _party true)
        (goto _label Break)))
    (:Completed
      (Variables|/Game/Blueprints/PartySystem.PartySystem_C|SetAnyMonsterAlive _party false)
      (Default|EndRound (Variables|Default|GetRoundManager)))))

(fn SetCurrentAction
  (params (GameSlot :type BP%20Monster%20Object%20Reference))
  (bind _selectedmoveindex (Variables|/Game/Blueprints/MonsterGameSlots/BP_Monster.BP_Monster_C|GetselectedMoveIndex GameSlot))
  (if (and (>= _selectedmoveindex 0) (<= _selectedmoveindex 3))
    (Variables|/Game/Blueprints/MonsterGameSlots/BP_Monster.BP_Monster_C|SetcurrentAction GameSlot "NewEnumerator0")
    (elif (!= (Variables|/Game/Blueprints/MonsterGameSlots/BP_Monster.BP_Monster_C|GetSelectedPartyIndex GameSlot) -1)
      (Variables|/Game/Blueprints/MonsterGameSlots/BP_Monster.BP_Monster_C|SetcurrentAction GameSlot "NewEnumerator1")
      (elif (!= (Variables|/Game/Blueprints/MonsterGameSlots/BP_Monster.BP_Monster_C|GetitemIndex GameSlot) -1)
        (Variables|/Game/Blueprints/MonsterGameSlots/BP_Monster.BP_Monster_C|SetcurrentAction GameSlot "NewEnumerator2")
        (else
          (Variables|/Game/Blueprints/MonsterGameSlots/BP_Monster.BP_Monster_C|SetcurrentAction GameSlot "NewEnumerator3")
          (Development|PrintString "Current Action Selection Issue "))))))

(fn CurrentActionSwitch
  (params (game%20slot :type BP%20Monster%20Object%20Reference))
  (switch Utilities|FlowControl|Switch|SwitchonActionType (Variables|/Game/Blueprints/MonsterGameSlots/BP_Monster.BP_Monster_C|GetcurrentAction game%20slot)
    (:NewEnumerator3
      (Development|PrintString "SELECTION NONE ERROR " true true "(R=1.000000,G=0.000000,B=0.237691,A=1.000000)" 5.0))
    (:NewEnumerator0
      (Default|AttackSelect game%20slot (Variables|/Game/Blueprints/MonsterGameSlots/BP_Monster.BP_Monster_C|GetselectedMoveIndex game%20slot)))
    (:NewEnumerator2
      (Development|PrintString "ITEM LOGIC HERE"))))
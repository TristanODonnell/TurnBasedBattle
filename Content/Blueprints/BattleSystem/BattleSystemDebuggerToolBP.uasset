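; Debug actor that exercises the monster battle system with test parties and shows results in a debug widget.
; After a short delay, BeginPlay fetches the widget from GameManager, loads both parties, initializes player and AI slots, then runs a status test.
; The test applies a chosen status, displays the player slot and runs end-turn twice, flagging it healed between.
; A separate event displays MoveCalculator damage inputs and results; ability checks are unwired.
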(event Custom|Game%20Slot%20Initialization
  (bind _player_slot (Variables|Default|GetPlayer%20Slot))
  (bind _ai_slot_ (Variables|Default|GetAI%20Slot%20))
  (bind _party (Variables|/Game/Blueprints/MonsterGameSlots/BP_Monster.BP_Monster_C|GetParty _ai_slot_))
  (bind _party_2 (Variables|/Game/Blueprints/MonsterGameSlots/BP_Monster.BP_Monster_C|GetParty _player_slot))
  ;[0.15 0.15 0.15 0.5] Slot Setup(see functions)
  (Default|SetSlotsArray (Variables|Default|Getbattlesystem))
  ;[0.15 0.15 0.15 0.5] Player Party Init
  (Default|SetMonsterInstArray _party_2) ; Add the data array to the instance array
  (Default|SetCurrentInst _party_2)
  (Default|StatSetup _player_slot _party_2) ; Set Slot Info for Player
  ;[0.15 0.15 0.15 0.5] AI Party Selection + Init
  (Default|SetMonsterInstArray _party) ; Add the data array to the instance array
  (Default|SetCurrentInst _party)
  (Default|StatSetup _ai_slot_ _party) ; Set Slot Info for AI
)

(event Custom|Set%20Party%20Data
  (Variables|/Game/Blueprints/PartySystem.PartySystem_C|SetMonsterDataArray (Variables|Default|GetPlayer%20Party) (Variables|Default|GetPlayer%20Party%20Test%20Array))
  (Variables|/Game/Blueprints/PartySystem.PartySystem_C|SetMonsterDataArray (Variables|Default|GetAI%20Party) (Variables|Default|GetAI%20Party%20Test%20Array%20)))

(event Custom|StatusTestDebugger
  (CallFunction|SetCurrentStatus)
  (Default|SetGameSlotDisplayText (Variables|Default|GetDebugBattleSystemWidget) (Variables|Default|GetPlayer%20Slot))
  (CallFunction|CallEndTurnPhase)
  (Development|PrintString "End Turn finished " true true "(R=0.000000,G=0.660000,B=1.000000,A=1.000000)" 5.0)
  (Variables|/Game/Blueprints/MonsterGameSlots/BP_Monster.BP_Monster_C|SetisHealed (Variables|Default|GetPlayer%20Slot) true)
  (CallFunction|CallEndTurnPhase))

(event Custom|CalculateMoveEffectsDebugger
  (bind _move_calculator (Variables|Default|GetMove%20Calculator))
  (bind _final_move_calculations (Default|CalculateMoveEffects _move_calculator (Variables|Default|GetAttacking%20Mon%20Attack) (Variables|Default|GetAttacking%20Mon%20Special%20Attack) (Variables|Default|GetAttacking%20Mon%20Type) (Variables|Default|GetDefending%20Mon%20Defence) (Variables|Default|GetDefending%20Mon%20Special%20Defence) (Variables|Default|GetDefending%20Mon%20Type) (Variables|Default|GetDebugAttackStruct)))
  (Default|SeMoveCalculationtDisplayText (Variables|Default|GetDebugBattleSystemWidget) (Variables|Default|GetDebugAttackStruct) _final_move_calculations (Variables|Default|GetAttacking%20Mon%20Type) (Variables|Default|GetDefending%20Mon%20Type) (Variables|/Game/Blueprints/BattleSystem/MoveCalculator.MoveCalculator_C|GetisStab _move_calculator))
  (Development|PrintString "Function is processing" true true "(R=0.968889,G=0.068014,B=1.000000,A=1.000000)" 5.0))

(event EventBeginPlay
  (Utilities|FlowControl|Delay 2.0)
  (bind _asgame_manager (Utilities|Casting|CastToGameManager (Game|GetGameInstance)))
  (Variables|Default|SetDebugBattleSystemWidget (Variables|/Game/Blueprints/UI/UIManager.UIManager_C|GetDebugBattleSystemWidget (Variables|/Game/Blueprints/GameManager.GameManager_C|GetUIManager _asgame_manager)))
  (CallFunction|SetPartyData)
  (CallFunction|GameSlotInitialization)
  (CallFunction|StatusTestDebugger))

(event Collision|EventActorBeginOverlap
  (params (OtherActor :type Actor%20Object%20Reference)))

(event EventTick
  (params (DeltaSeconds :type Float%20%28single-precision%29)))

(fn ConstructionScript)

(fn CallEndTurnPhase
  (Default|EndTurnEvent (Variables|Default|Getbattlesystem)))

(fn SetCurrentStatus
  (Default|TakeStatus (Variables|Default|GetPlayer%20Slot) (Variables|Default|GetStatusToTest)))
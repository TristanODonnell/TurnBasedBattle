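; AISelector picks the AI opponent's turn action in a monster battle: switch monsters or use a move.
; EvaluateTurnDecision switches when the player's type advantage reaches SwitchMinimum and the AI has two or more monsters alive.
; Living backups or current moves are scored against the player's monster using TypeMatchupDataTable effectiveness sums.
; EvaluateAction picks the top score, breaking ties randomly, and the action and index are written to AISlot.
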(event EventBeginPlay
  (Variables|Default|SetPlayer%20Party (Variables|/Game/Blueprints/MonsterGameSlots/BP_Monster.BP_Monster_C|GetParty (Variables|Default|GetPlayer%20Slot)))
  (Variables|Default|SetAIParty (Variables|/Game/Blueprints/MonsterGameSlots/BP_Monster.BP_Monster_C|GetParty (Variables|Default|GetAISlot)))
  (Variables|Default|SetMoveList "/Game/Blueprints/MoveData/MoveList.MoveList"))

(event Collision|EventActorBeginOverlap
  (params (OtherActor :type Actor%20Object%20Reference)))

(event EventTick
  (params (DeltaSeconds :type Float%20%28single-precision%29)))

(fn ConstructionScript)

(fn EvaluateTurnDecision
  (Development|PrintString "Evaluating Turn Decision " true true "(R=1.000000,G=1.000000,B=1.000000,A=1.000000)" 5.0)
  (bind _totalswitchscore (CallFunction|TypeAdvantageSwapCalculation (Variables|/Game/Blueprints/PartySystem.PartySystem_C|GetcurrentMonsterInst (Variables|Default|GetPlayer%20Party)) (Variables|/Game/Blueprints/PartySystem.PartySystem_C|GetcurrentMonsterInst (Variables|Default|GetAIParty)))) ; Check Type Advantage Between current Slots
  (Development|PrintString "type advantage current to current done " true true "(R=1.000000,G=1.000000,B=1.000000,A=1.000000)" 1e+01)
  ;[0.15 0.15 0.15 0.5] IF TRUE WE START SWITCH SELECTION
  (if (and (>= (Variables|/Game/Blueprints/PartySystem.PartySystem_C|GetAliveCount (Variables|Default|GetAIParty)) 2) (>= _totalswitchscore (Variables|Default|GetSwitchMinimum)))
    (CallFunction|EvaluateSwitchOptions)
    (Variables|/Game/Blueprints/MonsterGameSlots/BP_Monster.BP_Monster_C|SetcurrentAction (Variables|Default|GetAISlot) "NewEnumerator1")
    (else
      (CallFunction|EvaluateMoveChoice)
      (Variables|/Game/Blueprints/MonsterGameSlots/BP_Monster.BP_Monster_C|SetcurrentAction (Variables|Default|GetAISlot) "NewEnumerator0"))))

(fn TypeAdvantageSwapCalculation
  (params (AttackingMonster :type Monster%20Instance%20Structure) (DefendingMonster :type Monster%20Instance%20Structure))
  (bind _filteredtypestructarray (LocalVariables|GetFilteredTypeStructArray))
  (bind _effectivenesssum (LocalVariables|GetEffectivenessSum))
  (for _array_element (.monstertype AttackingMonster)
    (bind _returnvalue (Utilities|GetDataTableRow (Variables|Default|GetTypeMatchupDataTable) (Utilities|String|StringToName (Utilities|String|EnumtoString _array_element)))
      (:then
        (Development|PrintString "About to type advantage calc" true true "(R=0.979167,G=0.992917,B=1.000000,A=1.000000)" 1e+01)
        (for _array_element_2 (.Effectiveness (Utilities|Struct|BreakTypeChart _returnvalue))
          (if (Utilities|Array|ContainsItem (.monstertype DefendingMonster) (.DefendingType (Utilities|Struct|BreakEffectivenessEntry _array_element_2)))
            (Utilities|Array|Add _filteredtypestructarray _array_element_2)))
        (for _array_element_3 _filteredtypestructarray
          (Utilities|Array|Add _effectivenesssum (.effectiveness _array_element_3)))
        (for _array_element_4 _effectivenesssum
          (LocalVariables|SetTotalScore (+ _array_element_4 (LocalVariables|GetTotalScore))))
        (Development|PrintString (Utilities|String|ToString(Text) (Utilities|Text|FormatText "Total Local Score from current to current {score}" (LocalVariables|GetTotalScore))) true true "(R=1.000000,G=1.000000,B=1.000000,A=1.000000)" 1e+01)
        (return (LocalVariables|GetTotalScore))))))

(fn EvaluateSwitchOptions
  (bind _switchscorelocalmap (LocalVariables|GetSwitchScoreLocalMap))
  (bind _aiparty (Variables|Default|GetAIParty))
  (bind _currentmonsterinst (Variables|/Game/Blueprints/PartySystem.PartySystem_C|GetcurrentMonsterInst _aiparty))
  (Utilities|Map|Clear (LocalVariables|GetSwitchScoreLocalMap))
  (Utilities|Array|Clear (LocalVariables|GetvalidMonsterScores))
  (Utilities|Array|Clear (LocalVariables|GetValidBackupInstances))
  (Utilities|Array|Clear (LocalVariables|GetValidoriginalIndeces))
  ;[0.15 0.15 0.15 0.5] Determine Monsters in Party not Dead
  (Development|PrintString (Utilities|String|ToString(Text) (Utilities|Text|FormatText "Current Monster is dead: {bool}" (.isdead _currentmonsterinst))) true true "(R=1.000000,G=1.000000,B=1.000000,A=1.000000)" 1e+01)
  (for (_array_element _array_index) (Variables|/Game/Blueprints/PartySystem.PartySystem_C|GetMonsterInstanceArray (Variables|Default|GetAIParty))
    (if (Math|Boolean|ANDBoolean (!= (.MonsterID (Utilities|Struct|BreakMonsterInstance _array_element)) (.monsterid _currentmonsterinst)) (> (.MonsterID (Utilities|Struct|BreakMonsterInstance _array_element)) 0) (not (.isDead (Utilities|Struct|BreakMonsterInstance _array_element))))
      (Development|PrintString (Utilities|String|ToString(Text) (Utilities|Text|FormatText "{monster} is valid?  is dead =  {boolval}" (.Name (Utilities|Struct|BreakMonsterInstance _array_element)) (.isDead (Utilities|Struct|BreakMonsterInstance _array_element)))) true true "(R=0.000000,G=0.660000,B=1.000000,A=1.000000)" 3e+01)
      (Utilities|Array|Add (LocalVariables|GetValidBackupInstances) _array_element)
      (Utilities|Array|Add (LocalVariables|GetValidoriginalIndeces) _array_index)))
  (for _array_element_2 (LocalVariables|GetValidBackupInstances)
    (bind _totalswitchscore (CallFunction|TypeAdvantageSwapCalculation _array_element_2 (Variables|/Game/Blueprints/PartySystem.PartySystem_C|GetcurrentMonsterInst (Variables|Default|GetPlayer%20Party))))
    ;[0.15 0.15 0.15 0.5] Calculating Total Switch Scores
    (Utilities|Array|Add (LocalVariables|GetvalidMonsterScores) _totalswitchscore))
  (for _array_element_3 (LocalVariables|GetvalidMonsterScores)
    (Development|PrintString (Utilities|String|ToString(Text) (Utilities|Text|FormatText "Monster Score {score}" _array_element_3)) true true "(R=1.000000,G=1.000000,B=1.000000,A=1.000000)" 1e+01))
  ;[0.15 0.15 0.15 0.5] Add Switch Values to Corresponding Map based on original indeces
  (for (_array_element_4 _array_index_2) (LocalVariables|GetValidoriginalIndeces)
    (Utilities|Map|Add _switchscorelocalmap _array_element_4 (Utilities|Array|Get(acopy) (LocalVariables|GetvalidMonsterScores) _array_index_2)))
  (bind _keys (Utilities|Map|Keys _switchscorelocalmap))
  (for _array_element_5 _keys
    (Development|PrintString (Utilities|String|ToString(Text) (Utilities|Text|FormatText "Original Index value: {index} and valid monster score {score}" _array_element_5 (.Value (Utilities|Map|Find _switchscorelocalmap _array_element_5)))) true true "(R=0.860000,G=0.777534,B=0.000000,A=1.000000)" 1e+01))
  (bind _selectedindex (CallFunction|EvaluateAction _switchscorelocalmap))
  (Development|PrintString (Utilities|String|ToString(Text) (Utilities|Text|FormatText "Selected index {index}" _selectedindex)) true true "(R=0.860000,G=0.777534,B=0.000000,A=1.000000)" 1e+01)
  (Variables|Default|SetselectedaiIndex _selectedindex)
  (bind _output_get (Variables|/Game/Blueprints/MonsterGameSlots/BP_Monster.BP_Monster_C|SetSelectedPartyIndex (Variables|Default|GetAISlot) _selectedindex))
  (Development|PrintString (Utilities|String|ToString(Text) (Utilities|Text|FormatText "Selected Party index is : {index}" _output_get)) true true "(R=1.000000,G=1.000000,B=1.000000,A=1.000000)" 1e+01))

(fn TypeAdvantageMoveCalculation
  (params (Attacker%20%28AI%29 :type Monster%20Instance%20Structure) (Defender%20%28Player%29 :type Monster%20Instance%20Structure))
  (bind _filteredtypestructarray (LocalVariables|GetFilteredTypeStructArray))
  (bind _effectivenesssum (LocalVariables|GeteffectivenessSum))
  (Development|PrintString "Starting Calculation type advtange" true true "(R=1.000000,G=1.000000,B=1.000000,A=1.000000)" 1e+01)
  (Utilities|Map|Clear (Variables|Default|GetMoveScoreMap))
  (for (_array_element _array_index) (.currentmoveset Attacker%20%28AI%29)
    (bind _returnvalue (Utilities|GetDataTableRow (Variables|Default|GetMoveList) (Utilities|String|StringToName (Utilities|String|EnumtoString _array_element)))
      (:then
        (bind _returnvalue_2 (Utilities|GetDataTableRow (Variables|Default|GetTypeMatchupDataTable) (Utilities|String|StringToName (Utilities|String|EnumtoString (.userMoveType (Utilities|Struct|BreakMoveStruct _returnvalue)))))
          (:then
            (for _array_element_2 (.Effectiveness (Utilities|Struct|BreakTypeChart _returnvalue_2))
              (if (Utilities|Array|ContainsItem (.monstertype Defender%20%28Player%29) (.DefendingType (Utilities|Struct|BreakEffectivenessEntry _array_element_2)))
                (Utilities|Array|Add _filteredtypestructarray _array_element_2)))
            (for _array_element_3 _filteredtypestructarray
              (Utilities|Array|Add _effectivenesssum (.effectiveness _array_element_3)))
            (Utilities|Array|Clear _filteredtypestructarray)
            (for _array_element_4 _effectivenesssum
              (bind _output_get (LocalVariables|SetTotalMoveScore (+ _array_element_4 (LocalVariables|GetTotalMoveScore)))))
            (Utilities|Map|Add (Variables|Default|GetMoveScoreMap) _array_index (LocalVariables|GetTotalMoveScore))
            (Development|PrintString (Utilities|String|ToString(Text) (Utilities|Text|FormatText "Total Score {score}" _output_get)) true true "(R=1.000000,G=1.000000,B=1.000000,A=1.000000)" 1e+01)
            (Utilities|Array|Clear _effectivenesssum)
            (LocalVariables|SetTotalMoveScore 0.0))
          (:RowNotFound
            (Development|PrintString "ROW NOT FOUND" true true "(R=1.000000,G=0.000000,B=0.229527,A=1.000000)" 1e+01))))
      (:RowNotFound
        (Development|PrintString "ROW NOT FOUND" true true "(R=1.000000,G=0.000000,B=0.229527,A=1.000000)" 1e+01)))))

(fn EvaluateMoveChoice
  (CallFunction|TypeAdvantageMoveCalculation (Variables|/Game/Blueprints/PartySystem.PartySystem_C|GetcurrentMonsterInst (Variables|Default|GetAIParty)) (Variables|/Game/Blueprints/PartySystem.PartySystem_C|GetcurrentMonsterInst (Variables|Default|GetPlayer%20Party)))
  (bind _selectedindex (CallFunction|EvaluateAction (Variables|Default|GetMoveScoreMap)))
  (bind _output_get (Variables|/Game/Blueprints/MonsterGameSlots/BP_Monster.BP_Monster_C|SetselectedMoveIndex (Variables|Default|GetAISlot) _selectedindex))
  (Development|PrintString (Utilities|String|ToString(Text) (Utilities|Text|FormatText "Final selected index {int}" _output_get)) true true "(R=1.000000,G=1.000000,B=1.000000,A=1.000000)" 1e+01))

(fn EvaluateAction
  (params (ScoreMap :type Map%20of%20Integers%20to%20Reals))
  (bind _tiedindexes (LocalVariables|GetTiedIndexes))
  (Utilities|Array|Clear (LocalVariables|GetTiedIndexes))
  ;[0.15 0.15 0.15 0.5] Determine Highest Point Switch Option
  (bind _keys (Utilities|Map|Keys ScoreMap))
  (for _array_element _keys
    (if (> (.Value (Utilities|Map|Find ScoreMap _array_element)) (LocalVariables|GetMaxScore))
      (Development|PrintString "True for if value is greater than max score" true true "(R=0.840000,G=0.172603,B=0.000000,A=1.000000)" 1e+01)
      (bind _output_get (LocalVariables|SetMaxScore (.Value (Utilities|Map|Find ScoreMap _array_element))))
      (bind _output_get_2 (LocalVariables|SetMaxIndex _array_element))
      (Utilities|Array|Clear (LocalVariables|GetTiedIndexes))
      (Utilities|Array|Add (LocalVariables|GetTiedIndexes) _array_element)
      (Development|PrintString (Utilities|String|ToString(Text) (Utilities|Text|FormatText "Max Score {score} and max index {index}" _output_get _output_get_2)) true true "(R=0.840000,G=0.172603,B=0.000000,A=1.000000)" 1e+01)
      (else
        (Development|PrintString "index is false, tied" true true "(R=0.840000,G=0.172603,B=0.000000,A=1.000000)" 1e+01)
        (if (== (.Value (Utilities|Map|Find ScoreMap _array_element)) (LocalVariables|GetMaxScore))
          (Utilities|Array|Add (LocalVariables|GetTiedIndexes) _array_element)))))
  ;[0.15 0.15 0.15 0.5] Set Chosen Index inside AISlot
  (if (> (Utilities|Array|Length (LocalVariables|GetTiedIndexes)) 0)
    (Development|PrintString "tied indexes greater than 0 " true true "(R=0.840000,G=0.172603,B=0.000000,A=1.000000)" 1e+01)
    (bind _output_get_3 (LocalVariables|Setfinal%20index (Utilities|Array|Get(acopy) _tiedindexes (Math|Random|RandomIntegerinRange 0 (- (Utilities|Array|Length _tiedindexes) 1)))))
    (Development|PrintString (Utilities|String|ToString(Text) (Utilities|Text|FormatText "Selected index finish is {index}" _output_get_3)) true true "(R=0.840000,G=0.172603,B=0.000000,A=1.000000)" 1e+01)
    (return _output_get_3)
    (else
      (return (LocalVariables|GetMaxIndex)))))
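; AbilityManager resolves monster abilities in the battle system through one check function per battle trigger.
; Each check switches on a game slot's CurrentAbility and edits the user's or opponent's slot directly: stats, status, immunity or ability.
; Healing, damage, turn start, status, attack and slot entry have effects; turn end, item use, stat change and nullify are empty.
; Oblivion's reset of opponent stats leaves Speed unchanged because that node never runs.
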(event EventBeginPlay)

(event Collision|EventActorBeginOverlap
  (params (OtherActor :type Actor%20Object%20Reference)))

(event EventTick
  (params (DeltaSeconds :type Float%20%28single-precision%29)))

(fn ConstructionScript)

(fn OnHealedAbilityCheck
  (params (Game%20Slot%20 :type BP%20Monster%20Object%20Reference))
  (switch Utilities|FlowControl|Switch|SwitchonEMonsterAbility (Variables|/Game/Blueprints/MonsterGameSlots/BP_Monster.BP_Monster_C|GetcurrentAbility Game%20Slot%20)
    (:NewEnumerator9
      (Default|TakeStatChange Game%20Slot%20 0.0 1.05 1.05 1.05 1.05 1.05))))

(fn OnDamagedAbilityCheck
  (params (DefendingGameSlot :type BP%20Monster%20Object%20Reference) (AttackerGameSlot :type BP%20Monster%20Object%20Reference))
  (switch Utilities|FlowControl|Switch|SwitchonEMonsterAbility (Variables|/Game/Blueprints/MonsterGameSlots/BP_Monster.BP_Monster_C|GetcurrentAbility DefendingGameSlot)
    (:NewEnumerator1
      (if (<= (Variables|/Game/Blueprints/MonsterGameSlots/BP_Monster.BP_Monster_C|GetcurrentHealth DefendingGameSlot) (* (Variables|/Game/Blueprints/MonsterGameSlots/BP_Monster.BP_Monster_C|GetmaxHealth DefendingGameSlot) 0.2))
        (Variables|/Game/Blueprints/MonsterGameSlots/BP_Monster.BP_Monster_C|SetisImmune DefendingGameSlot true)
        (Variables|/Game/Blueprints/MonsterGameSlots/BP_Monster.BP_Monster_C|SetisImmuneCounter DefendingGameSlot 3)))
    (:NewEnumerator3
      (Default|TakeStatus AttackerGameSlot "NewEnumerator1"))))

(fn OnStartTurnAbilityCheck
  (params (Ability%20User :type BP%20Monster%20Object%20Reference) (Defender :type BP%20Monster%20Object%20Reference))
  (switch Utilities|FlowControl|Switch|SwitchonEMonsterAbility (Variables|/Game/Blueprints/MonsterGameSlots/BP_Monster.BP_Monster_C|GetcurrentAbility Ability%20User)
    (:NewEnumerator4
      (if (Variables|/Game/Blueprints/MonsterGameSlots/BP_Monster.BP_Monster_C|GetisActive Ability%20User)
        (Variables|/Game/Blueprints/MonsterGameSlots/BP_Monster.BP_Monster_C|SetcurrentAbility Defender "NewEnumerator10")))
    (:NewEnumerator7
      (if (>= (Variables|/Game/Blueprints/MonsterGameSlots/BP_Monster.BP_Monster_C|GetcurrentHealth Ability%20User) (* (Variables|/Game/Blueprints/MonsterGameSlots/BP_Monster.BP_Monster_C|GetmaxHealth Ability%20User) 0.8))
        (Variables|/Game/Blueprints/MonsterGameSlots/BP_Monster.BP_Monster_C|SetIsMagnitude Ability%20User true)))
    (:NewEnumerator8
      (Variables|/Game/Blueprints/MonsterGameSlots/BP_Monster.BP_Monster_C|SetcurrentSpeed Defender (* (Variables|/Game/Blueprints/MonsterGameSlots/BP_Monster.BP_Monster_C|GetcurrentSpeed Defender) 0.9)))))

(fn OnEndTurnAbilityCheck
  (params (Ability%20User :type BP%20Monster%20Object%20Reference) (Defending%20Slot :type BP%20Monster%20Object%20Reference)))

(fn OnItemUsedAbilityCheck)

(fn OnStatChangedAbilityCheck)

(fn OnAbilityNullifiedAbilityCheck)

(fn OnStatusGivenAbilityCheck
  (params (GameSLot :type BP%20Monster%20Object%20Reference))
  (switch Utilities|FlowControl|Switch|SwitchonEMonsterAbility (Variables|/Game/Blueprints/MonsterGameSlots/BP_Monster.BP_Monster_C|GetcurrentAbility GameSLot)
    (:NewEnumerator0
      (Variables|/Game/Blueprints/MonsterGameSlots/BP_Monster.BP_Monster_C|SethasStatus GameSLot false))))

(fn OnAttackPerformedAbilityCheck
  (params (GameSlot :type BP%20Monster%20Object%20Reference))
  (switch Utilities|FlowControl|Switch|SwitchonEMonsterAbility (Variables|/Game/Blueprints/MonsterGameSlots/BP_Monster.BP_Monster_C|GetcurrentAbility GameSlot)
    (:NewEnumerator5
      (Variables|/Game/Blueprints/MonsterGameSlots/BP_Monster.BP_Monster_C|SetisStatChangeImmune GameSlot true))))

(fn OnEnterGameSlotAbilityCheck
  (params (EnteringGameSlot :type BP%20Monster%20Object%20Reference) (Defending%20Game%20Slot :type BP%20Monster%20Object%20Reference))
  (bind _party (Variables|/Game/Blueprints/MonsterGameSlots/BP_Monster.BP_Monster_C|GetParty Defending%20Game%20Slot))
  (bind _currentmonsterinst (Variables|/Game/Blueprints/PartySystem.PartySystem_C|GetcurrentMonsterInst _party))
  (switch Utilities|FlowControl|Switch|SwitchonEMonsterAbility (Variables|/Game/Blueprints/MonsterGameSlots/BP_Monster.BP_Monster_C|GetcurrentAbility EnteringGameSlot)
    (:NewEnumerator6
      (Variables|/Game/Blueprints/MonsterGameSlots/BP_Monster.BP_Monster_C|SetcurrentAttack Defending%20Game%20Slot (.currentattack _currentmonsterinst))
      (Variables|/Game/Blueprints/MonsterGameSlots/BP_Monster.BP_Monster_C|SetcurrentSpecAttack Defending%20Game%20Slot (.currentspecattack _currentmonsterinst))
      (Variables|/Game/Blueprints/MonsterGameSlots/BP_Monster.BP_Monster_C|SetcurrentDefence Defending%20Game%20Slot (.currentdefence _currentmonsterinst))
      (Variables|/Game/Blueprints/MonsterGameSlots/BP_Monster.BP_Monster_C|SetcurrentSpecDefence Defending%20Game%20Slot (.currentspecdefence _currentmonsterinst)))))
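; Party system actor that holds a party of monsters as runtime instances and tracks which one is current.
; SetMonsterInstArray turns each valid monster data entry into an instance with copied stats, moveset, type, ability, visual and a random, not necessarily unique ID.
; SetCurrentInst selects an instance by index, with debug prints, and EmptyDataArray clears the source data.
; The event graph runs nothing itself, and EndRound is an empty stub.
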(event EventBeginPlay)

(event Collision|EventActorBeginOverlap
  (params (OtherActor :type Actor%20Object%20Reference)))

(event EventTick
  (params (DeltaSeconds :type Float%20%28single-precision%29)))

(fn ConstructionScript)

(fn SetMonsterInstArray
  (for _array_element (Variables|Default|GetMonsterDataArray)
    (if (Utilities|IsValid _array_element)
      (Development|PrintString "Trying to populate")
      (bind _int_created (CallFunction|SetID))
      (Utilities|Array|Add (Variables|Default|GetMonsterInstanceArray) (Utilities|Struct|MakeMonsterInstance (Variables|/Game/Blueprints/MonsterDataAssets/BP_MonsterDataAsset.BP_MonsterDataAsset_C|GetName _array_element) (Variables|/Game/Blueprints/MonsterDataAssets/BP_MonsterDataAsset.BP_MonsterDataAsset_C|GetHealth _array_element) (Variables|/Game/Blueprints/MonsterDataAssets/BP_MonsterDataAsset.BP_MonsterDataAsset_C|GetHealth _array_element) (Variables|/Game/Blueprints/MonsterDataAssets/BP_MonsterDataAsset.BP_MonsterDataAsset_C|GetAttack _array_element) (Variables|/Game/Blueprints/MonsterDataAssets/BP_MonsterDataAsset.BP_MonsterDataAsset_C|GetspecAttack _array_element) (Variables|/Game/Blueprints/MonsterDataAssets/BP_MonsterDataAsset.BP_MonsterDataAsset_C|GetDefence _array_element) (Variables|/Game/Blueprints/MonsterDataAssets/BP_MonsterDataAsset.BP_MonsterDataAsset_C|GetspecDefence _array_element) (Variables|/Game/Blueprints/MonsterDataAssets/BP_MonsterDataAsset.BP_MonsterDataAsset_C|GetSpeed _array_element) (Variables|/Game/Blueprints/MonsterDataAssets/BP_MonsterDataAsset.BP_MonsterDataAsset_C|GetMoveset _array_element) (Variables|/Game/Blueprints/MonsterDataAssets/BP_MonsterDataAsset.BP_MonsterDataAsset_C|GetMonssterType _array_element) (Variables|/Game/Blueprints/MonsterDataAssets/BP_MonsterDataAsset.BP_MonsterDataAsset_C|GetAbility _array_element) (Variables|/Game/Blueprints/MonsterDataAssets/BP_MonsterDataAsset.BP_MonsterDataAsset_C|GetMonsterVisual _array_element) false _int_created))
      (else
        (Development|PrintString "NO MONSTER ASSIGNED" true true "(R=1.000000,G=0.016703,B=0.000000,A=1.000000)" 1e+01)))))

(fn SetCurrentInst
  (params (NewArrayInt :type Integer))
  (bind _monsterinstancearray (Variables|Default|GetMonsterInstanceArray))
  (bind _output (Utilities|Array|Get(acopy) _monsterinstancearray NewArrayInt))
  (Development|PrintString (Utilities|String|ToString(Text) (Utilities|Text|FormatText "Monster grabbed from Index {monster}" (.Name (Utilities|Struct|BreakMonsterInstance _output)))) true true "(R=1.000000,G=1.000000,B=1.000000,A=1.000000)" 1e+01)
  (bind _output_get (Variables|Default|SetcurrentMonsterInst _output))
  (Variables|Default|SetCurrentArrayIndex NewArrayInt)
  (Development|PrintString (Utilities|String|ToString(Text) (Utilities|Text|FormatText "New Current inst is {monster} " (.name _output_get))) true true "(R=1.000000,G=1.000000,B=1.000000,A=1.000000)" 1e+01))

(fn EmptyDataArray
  (Utilities|Array|Clear (Variables|Default|GetMonsterDataArray)))

(fn EndRound)

(fn SetID
  (return (Math|Random|RandomIntegerinRange 1 50000)))
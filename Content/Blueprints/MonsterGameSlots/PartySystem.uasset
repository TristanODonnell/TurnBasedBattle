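; Party system actor that holds a team of monsters and tracks the current one.
; SetMonsterInstArray turns monster data entries into runtime instance structs with random IDs and counts them alive, while SetCurrentInst selects the current monster by index.
; AddExp triggers LevelUp at the threshold, scaling stats and the next experience requirement; GiveXP derives a reward from the current monster's level.
; SetPartyMultiplier raises party levels using RoundManager's round and multiplier.
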(event EventBeginPlay)

(event Collision|EventActorBeginOverlap
  (params (OtherActor :type Actor%20Object%20Reference)))

(event EventTick
  (params (DeltaSeconds :type Float%20%28single-precision%29)))

(fn ConstructionScript)

(fn SetMonsterInstArray
  (Utilities|Array|Clear (Variables|Default|GetMonsterInstanceArray))
  (for _array_element (Variables|Default|GetMonsterDataArray)
    (if (Utilities|IsValid _array_element)
      (Development|PrintString "Trying to populate")
      (bind _int_created (CallFunction|SetID))
      (Utilities|Array|Add (Variables|Default|GetMonsterInstanceArray) (Utilities|Struct|MakeMonsterInstance (Variables|/Game/Blueprints/MonsterDataAssets/BP_MonsterDataAsset.BP_MonsterDataAsset_C|GetName _array_element) (Variables|/Game/Blueprints/MonsterDataAssets/BP_MonsterDataAsset.BP_MonsterDataAsset_C|GetHealth _array_element) (Variables|/Game/Blueprints/MonsterDataAssets/BP_MonsterDataAsset.BP_MonsterDataAsset_C|GetHealth _array_element) (Variables|/Game/Blueprints/MonsterDataAssets/BP_MonsterDataAsset.BP_MonsterDataAsset_C|GetAttack _array_element) (Variables|/Game/Blueprints/MonsterDataAssets/BP_MonsterDataAsset.BP_MonsterDataAsset_C|GetspecAttack _array_element) (Variables|/Game/Blueprints/MonsterDataAssets/BP_MonsterDataAsset.BP_MonsterDataAsset_C|GetDefence _array_element) (Variables|/Game/Blueprints/MonsterDataAssets/BP_MonsterDataAsset.BP_MonsterDataAsset_C|GetspecDefence _array_element) (Variables|/Game/Blueprints/MonsterDataAssets/BP_MonsterDataAsset.BP_MonsterDataAsset_C|GetSpeed _array_element) (Variables|/Game/Blueprints/MonsterDataAssets/BP_MonsterDataAsset.BP_MonsterDataAsset_C|GetMoveset _array_element) (Variables|/Game/Blueprints/MonsterDataAssets/BP_MonsterDataAsset.BP_MonsterDataAsset_C|GetMonssterType _array_element) (Variables|/Game/Blueprints/MonsterDataAssets/BP_MonsterDataAsset.BP_MonsterDataAsset_C|GetAbility _array_element) (Variables|/Game/Blueprints/MonsterDataAssets/BP_MonsterDataAsset.BP_MonsterDataAsset_C|GetMonsterVisual _array_element) false _int_created false "(StatusEffect_2_C5233A014D99199AAC621A85606DB6B6=NewEnumerator7,Duration_9_C2C90E4A4EC83EA891B89D9E0AC4B64F=0,StatusEffectPercentage_23_2D33FE85467CDC7EB5A1B0BF4865A302=0.000000,DamagePercentage_18_F121804F4D6129ECA4F7738E19BCEA8F=0.000000,StatModifierPercentage_19_BB4021ED4EA02A9E960271992ED79A16=0.000000,DamageType_22_760A002242693683F3CC1E9C4155F192=NewEnumerator2,hasTurnCount_25_0CD5AA164BA968FA6E3012B98DAB0C9F=False)" 5 0 150 10 (Variables|/Game/Blueprints/MonsterDataAssets/BP_MonsterDataAsset.BP_MonsterDataAsset_C|GetMonsterSound _array_element)))
      (Variables|Default|SetAliveCount (+ (Variables|Default|GetAliveCount) 1))
      (else
        (Development|PrintString "NO MONSTER ASSIGNED" true true "(R=1.000000,G=0.016703,B=0.000000,A=1.000000)" 1e+01)))))

(fn SetCurrentInst
  (params (NewArrayInt :type Integer))
  (bind _monsterinstancearray (Variables|Default|GetMonsterInstanceArray))
  (bind _output (Utilities|Array|Get(acopy) _monsterinstancearray NewArrayInt))
  (Development|PrintString (Utilities|String|ToString(Text) (Utilities|Text|FormatText "Monster grabbed from Index {monster}" (.Name (Utilities|Struct|BreakMonsterInstance _output)))) true true "(R=1.000000,G=1.000000,B=1.000000,A=1.000000)" 1e+01)
  (bind _output_get (Variables|Default|SetcurrentMonsterInst _output))
  (Variables|Default|SetCurrentArrayIndex NewArrayInt)
  (Development|PrintString (Utilities|String|ToString(Text) (Utilities|Text|FormatText "New Current inst is {monster} " (.name _output_get))) true true "(R=1.000000,G=1.000000,B=1.000000,A=1.000000)" 1e+01))

(fn EmptyDataArray
  (Utilities|Array|Clear (Variables|Default|GetMonsterDataArray)))

(fn EndRound)

(fn SetID
  (return (Math|Random|RandomIntegerinRange 1 50000)))

(fn LevelUp
  (params (MonsterInstance :type Monster%20Instance%20Structure))
  (bind (_name _maxhealth _currenthealth _currentattack _currentspecattack _currentdefence _currentspecdefence _currentspeed _currentmoveset _monstertype _monsterability _monstervisual _isdead _monsterid _hasstatus _currentstatus _currentlevel _currentexp _nextlevelexp _baseexp) (Utilities|Struct|BreakMonsterInstance MonsterInstance))
  (bind _returnvalue (+ _currentlevel 1))
  (Utilities|Struct|SetmembersinMonsterInstance MonsterInstance (* _maxhealth (Variables|Default|GetLevelUpMultiplier)) (* _currenthealth (Variables|Default|GetLevelUpMultiplier)) (* _currentattack (Variables|Default|GetLevelUpMultiplier)) (* _currentspecattack (Variables|Default|GetLevelUpMultiplier)) (* _currentdefence (Variables|Default|GetLevelUpMultiplier)) (* _currentspecdefence (Variables|Default|GetLevelUpMultiplier)) (* _currentspeed (Variables|Default|GetLevelUpMultiplier)) _returnvalue (- _currentexp _nextlevelexp) (+ _baseexp (* (Variables|Default|GetIncremement) _returnvalue))))

(fn AddExp
  (params (MonsterInstance :type Monster%20Instance%20Structure) (Exp%20toAdd :type Integer))
  (bind _structout (Utilities|Struct|SetmembersinMonsterInstance MonsterInstance (+ (.currentexp (Variables|Default|GetcurrentMonsterInst)) Exp%20toAdd)))
  (if (>= (.currentExp (Utilities|Struct|BreakMonsterInstance _structout)) (.nextLevelExp (Utilities|Struct|BreakMonsterInstance _structout)))
    (CallFunction|LevelUp _structout)
    (return true)
    (else
      (return false))))

(fn GiveXP
  (return (* (.CurrentLevel (Utilities|Struct|BreakMonsterInstance (Variables|Default|GetcurrentMonsterInst))) (Variables|Default|GetXpGivenMultiplier))))

(fn SetPartyMultiplier
  (bind _roundmanager (Variables|Default|GetRoundManager))
  (for _array_element (Variables|Default|GetMonsterInstanceArray)
    (Utilities|Struct|SetmembersinMonsterInstance _array_element (+ (.CurrentLevel (Utilities|Struct|BreakMonsterInstance _array_element)) (* (Variables|/Game/Blueprints/RoundManager.RoundManager_C|GetcurrentRound _roundmanager) (Variables|/Game/Blueprints/RoundManager.RoundManager_C|GetLevelMultiplier _roundmanager))))))
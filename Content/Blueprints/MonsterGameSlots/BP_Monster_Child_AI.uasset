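; BP_Monster_Child_AI is a child monster Blueprint that makes random choices for an AI-controlled monster in battle.
; GetIndexSelection picks a random move index from the current moveset.
; GetSwitchIndex loops until a random party roll finds a living monster, but sets SelectedPartyIndex from a separate roll, so it can land on a dead one, and returns 0.
; Its event graph holds only disabled parent-call stubs.
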(event EventBeginPlay
  (|CallParentFunction) ; This node is disabled and will not be called.\nDrag off pins to build functionality.
)

(event Collision|EventActorBeginOverlap
  (params (OtherActor :type Actor%20Object%20Reference))
  (|CallParentFunction OtherActor) ; This node is disabled and will not be called.\nDrag off pins to build functionality.
)

(event EventTick
  (params (DeltaSeconds :type Float%20%28single-precision%29))
  (|CallParentFunction DeltaSeconds) ; This node is disabled and will not be called.\nDrag off pins to build functionality.
)

(fn ConstructionScript
  (|CallParentFunction))

(fn GetIndexSelection
  (Variables|Default|SetselectedMoveIndex (Math|Random|RandomIntegerinRange 0 (- (Utilities|Array|Length (Variables|Default|GetcurrentMoveset)) 1)))
  (return))

(fn GetSwitchIndex
  (bind _party (Variables|Default|GetParty))
  (bind _monsterinstancearray (Variables|/Game/Blueprints/PartySystem.PartySystem_C|GetMonsterInstanceArray _party))
  (bind _returnvalue (Utilities|Array|Length _monsterinstancearray))
  (bind _returnvalue_2 (- _returnvalue 1))
  (bind _returnvalue_3 (Math|Random|RandomIntegerinRange 0 _returnvalue_2))
  (LocalVariables|SetFoundAliveMonster false)
  (while (== (LocalVariables|GetFoundAliveMonster) false)
    (if (not (.isDead (Utilities|Struct|BreakMonsterInstance (Utilities|Array|Get(acopy) _monsterinstancearray _returnvalue_3))))
      (Variables|Default|SetSelectedPartyIndex _returnvalue_3)
      (LocalVariables|SetFoundAliveMonster true)))
  (return 0))
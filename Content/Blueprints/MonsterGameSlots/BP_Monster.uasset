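; BP_Monster is a battle monster actor that represents the active member of a party in a monster battle game.
; StatSetup copies stats, moveset and mesh from the party's current monster instance, resetting health to max.
; SwapMonster writes the moveset and health (into the attack field) back to that instance, then reloads from the selected member.
; TakeDamage respects blocking, AttackSelect picks a move, and stat change, status, reset and selection getters are unfinished.
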(event EventBeginPlay)

(event Collision|EventActorBeginOverlap
  (params (OtherActor :type Actor%20Object%20Reference)))

(event EventTick
  (params (DeltaSeconds :type Float%20%28single-precision%29)))

(fn ConstructionScript)

(fn StatSetup
  (params (UserParty :type Party%20System%20Object%20Reference))
  (bind _currentmonsterinst (Variables|/Game/Blueprints/PartySystem.PartySystem_C|GetcurrentMonsterInst UserParty))
  (bind (_name _currenthealth _currentattack _currentspecattack _currentdefence _currentspecdefence _currentspeed _currentmoveset _monstertype _ability _monstervisual _isdead _maxhealth) (Utilities|Struct|BreakMonsterInstance _currentmonsterinst))
  (Development|PrintString "STARTING STAT SET UP " true true "(R=0.719543,G=0.000000,B=1.000000,A=1.000000)" 1e+01)
  (bind _output_get (Variables|Default|SetmaxHealth (Math|Conversions|ToFloat(Integer) (Math|Float|Truncate _maxhealth))))
  (Variables|Default|SetcurrentHealth _output_get)
  (Variables|Default|SetmonsterName _name)
  (Variables|Default|SetcurrentAttack _currentattack)
  (Variables|Default|SetcurrentSpecAttack _currentspecattack)
  (Variables|Default|SetcurrentDefence _currentdefence)
  (Variables|Default|SetcurrentSpecDefence _currentspecdefence)
  (Variables|Default|SetcurrentSpeed _currentspeed)
  (Variables|Default|SetMonsterType _monstertype)
  (Variables|Default|SetcurrentMoveset _currentmoveset)
  (bind _output_get_2 (Variables|Default|SetMonster%20Visual _monstervisual))
  (Components|StaticMesh|SetStaticMesh (Variables|Default|GetMonsterVisual%20component) _output_get_2)
  (Development|PrintString (Utilities|GetDisplayName _output_get_2) true true "(R=0.126427,G=1.000000,B=0.138753,A=1.000000)" 5.0))

(fn TakeStatChange
  (params (HealthMultiplier :type Float%20%28double-precision%29) (AttackMultiplier :type Float%20%28double-precision%29) (SpAttackMultiplier :type Float%20%28double-precision%29) (DefenceMultiplier :type Float%20%28double-precision%29) (SpecialDefenceMultiplier :type Float%20%28double-precision%29) (SpeedMultiplier :type Float%20%28double-precision%29)))

(fn TakeDamage
  (params (AttackDamageVal :type Integer))
  (if (not (Variables|Default|GetisBlockMove))
    (Variables|Default|SetcurrentHealth (- (Variables|Default|GetcurrentHealth) AttackDamageVal))))

(fn ResetStats)

(fn AttackSelect
  (params (SelectedIndex :type Integer))
  (Variables|Default|SetSelectedMove (Utilities|Array|Get(acopy) (Variables|Default|GetcurrentMoveset) SelectedIndex))
  (return))

(fn GetIndexSelection
  (return))

(fn GetSwitchIndex
  (return))

(fn SwapMonster
  (bind _party (Variables|Default|GetParty))
  (bind _party_2 (Variables|Default|GetParty))
  (if (Variables|/Game/Blueprints/PartySystem.PartySystem_C|GetAnyMonsterAlive _party_2)
    (bind _structout (Utilities|Struct|SetmembersinMonsterInstance (Variables|/Game/Blueprints/PartySystem.PartySystem_C|GetcurrentMonsterInst _party_2)))
    (|SetBy-RefVar (.currentattack _structout) (Variables|Default|GetcurrentHealth))
    (|SetBy-RefVar (.currentmoveset _structout) (Variables|Default|GetcurrentMoveset))
    (CallFunction|GetSwitchIndex)
    (Default|SetCurrentInst _party (Variables|Default|GetSelectedPartyIndex))
    (CallFunction|StatSetup _party)))

(fn TakeStatus)

(fn SetPartySystem
  (params (Party%20System :type Party%20System%20Object%20Reference))
  (Variables|Default|SetParty Party%20System))
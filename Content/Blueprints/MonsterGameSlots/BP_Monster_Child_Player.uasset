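; Player-side child of a monster Blueprint that receives the player's move and party-switch choices from the UI.
; After a two-second delay on BeginPlay, it gets the move and party selector widgets from the GameManager game instance's UIManager and binds to their selection events.
; A move pick stores the selected index, while a party pick stores the switch index and also sets the current action enum.
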(event Custom|handleswitchselected
  (bind _index (CallFunction|GetSwitchIndex))
  (Development|PrintString (Utilities|String|Append (Utilities|String|ToString(Integer) _index) "monster"))
  (Variables|Default|SetcurrentAction "NewEnumerator1"))

(event Custom|handleButtonSelected
  (CallFunction|GetIndexSelection)
  (Development|PrintString "Index Selected  "))

(event EventBeginPlay
  (|CallParentFunction)
  (Development|PrintString "Trying to load move")
  (Utilities|FlowControl|Delay 2.0)
  (bind _asgame_manager (Utilities|Casting|CastToGameManager (Game|GetGameInstance)))
  (bind _output_get (Variables|Default|SetMoveSelector (Variables|/Game/Blueprints/UI/UIManager.UIManager_C|GetMoveSelectorUI (Variables|/Game/Blueprints/GameManager.GameManager_C|GetUIManager _asgame_manager))))
  (EventDispatchers|BindEventtoOnButtonSelected _output_get (delegate Custom|handleButtonSelected))
  (bind _output_get_2 (Variables|Default|SetPartySelector (Variables|/Game/Blueprints/UI/UIManager.UIManager_C|GetPartySelectorUI (Variables|/Game/Blueprints/GameManager.GameManager_C|GetUIManager _asgame_manager))))
  (EventDispatchers|BindEventtoOnPartyButtonSelected _output_get_2 (delegate Custom|handleswitchselected)))

(fn ConstructionScript
  (|CallParentFunction))

(fn GetIndexSelection
  (Variables|Default|SetselectedMoveIndex (Variables|/Game/Blueprints/UI/BPMoveSelector.BPMoveSelector_C|GetcurrentIndex (Variables|Default|GetMoveSelector)))
  (return))

(fn GetSwitchIndex
  (bind _output_get (Variables|Default|SetSelectedPartyIndex (Variables|/Game/Blueprints/UI/PartySelector.PartySelector_C|GetcurrentIndex (Variables|Default|GetPartySelector))))
  (return _output_get))
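; BP_Monster_Child_Player is a player monster Blueprint that picks up move choices from the move selector UI.
; After the parent BeginPlay and a fixed delay, it gets the MoveSelectorUI through the GameManager game instance's UIManager and binds to its button-selected event.
; On selection, it copies the selector's current index into SelectedMoveIndex and prints a debug message, with no move execution in this graph.
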(event Custom|handleButtonSelected
  (CallFunction|GetIndexSelection)
  (Development|PrintString "Index Selected  "))

(event EventBeginPlay
  (|CallParentFunction)
  (Development|PrintString "Trying to load move")
  (Utilities|FlowControl|Delay 2.0)
  (bind _asgame_manager (Utilities|Casting|CastToGameManager (Game|GetGameInstance)))
  (bind _output_get (Variables|Default|SetMoveSelector (Variables|/Game/Blueprints/UIManager.UIManager_C|GetMoveSelectorUI (Variables|/Game/Blueprints/GameManager.GameManager_C|GetUIManager _asgame_manager))))
  (EventDispatchers|BindEventtoOnButtonSelected _output_get (delegate Custom|handleButtonSelected)))

(fn ConstructionScript
  (|CallParentFunction))

(fn GetIndexSelection
  (Variables|Default|SetselectedMoveIndex (Variables|/Game/Blueprints/BPMoveSelector.BPMoveSelector_C|GetcurrentIndex (Variables|Default|GetMoveSelector)))
  (return))
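; BP_BattleSystem is a Blueprint that manages a turn-based monster battle between a player slot and an enemy slot.
; On BeginPlay, LoadMonster calls StatSetup on both slots.
; TurnPhase sets CurrentTurn by comparing the slots' CurrentSpeed, with ties taking the same branch as a faster enemy.
; TurnPhase is not called within this Blueprint, and AttackPhase is an empty stub.
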(event EventBeginPlay
  (CallFunction|LoadMonster))

(event Collision|EventActorBeginOverlap
  (params (OtherActor :type Actor%20Object%20Reference)))

(event EventTick
  (params (DeltaSeconds :type Float%20%28single-precision%29)))

(fn ConstructionScript)

(fn LoadMonster
  (Default|StatSetup (Variables|Default|GetPlayerSlot))
  (Default|StatSetup (Variables|Default|GetEnemySlot)))

(fn TurnPhase
  (if (> (Variables|/Game/Blueprints/BP_Monster.BP_Monster_C|GetcurrentSpeed (Variables|Default|GetPlayerSlot)) (Variables|/Game/Blueprints/BP_Monster.BP_Monster_C|GetcurrentSpeed (Variables|Default|GetEnemySlot)))
    (Variables|Default|SetcurrentTurn "NewEnumerator0")
    (else
      (Variables|Default|SetcurrentTurn "NewEnumerator1"))))

(fn AttackPhase)
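; BP_Monster is a monster Blueprint that holds a monster's name and combat stats.
; StatSetup copies name, health, attack, defence and speed from MonsterData into current-value variables, or prints an error when no data is assigned.
; The moveset copy is disconnected, TakeDamage is an empty stub, and nothing in this Blueprint calls StatSetup.
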(event EventBeginPlay)

(event Collision|EventActorBeginOverlap
  (params (OtherActor :type Actor%20Object%20Reference)))

(event EventTick
  (params (DeltaSeconds :type Float%20%28single-precision%29)))

(fn ConstructionScript)

(fn StatSetup
  (bind _monsterdata (Variables|Default|GetMonsterData))
  (if (Utilities|IsValid _monsterdata)
    (Variables|Default|SetmonsterName (Variables|/Game/Blueprints/BP_MonsterDataAsset.BP_MonsterDataAsset_C|GetName _monsterdata))
    (Variables|Default|SetcurrentHealth (Variables|/Game/Blueprints/BP_MonsterDataAsset.BP_MonsterDataAsset_C|GetHealth _monsterdata))
    (Variables|Default|SetcurrentAttack (Variables|/Game/Blueprints/BP_MonsterDataAsset.BP_MonsterDataAsset_C|GetAttack _monsterdata))
    (Variables|Default|SetcurrentDefence (Variables|/Game/Blueprints/BP_MonsterDataAsset.BP_MonsterDataAsset_C|GetDefence _monsterdata))
    (Variables|Default|SetcurrentSpeed (Variables|/Game/Blueprints/BP_MonsterDataAsset.BP_MonsterDataAsset_C|GetSpeed _monsterdata))
    (else
      (Development|PrintString "NO MONSTER ASSIGNED" true true "(R=1.000000,G=0.016703,B=0.000000,A=1.000000)" 1e+01))))

(fn TakeDamage)
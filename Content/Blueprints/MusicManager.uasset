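; MusicManager Blueprint that plays a playlist of background songs as 2D sound, one after another in array order.
; On BeginPlay it caches each song's duration in SongLengths and starts the first track.
; A timer set to the current song's length calls PlayNextSong to advance the index.
; Past the last song the index resets to zero, but that branch plays nothing and sets no timer, so playback ends.
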(event Custom|PlayNextSong
  (bind _playlist (Variables|Default|GetPlaylist))
  (bind _output_get (Variables|Default|SetCurrentIndex (+ (Variables|Default|GetCurrentIndex) 1)))
  (if (>= _output_get (Utilities|Array|Length _playlist))
    (Variables|Default|SetCurrentIndex 0)
    (else
      (Audio|PlaySound2D (Utilities|Array|Get(acopy) _playlist (Variables|Default|GetCurrentIndex)) 1.0 1.0 0.0 0 0)
      (Utilities|Time|SetTimerbyEvent (delegate Custom|PlayNextSong) (Utilities|Array|Get(acopy) (Variables|Default|GetSongLengths) (Variables|Default|GetCurrentIndex))))))

(event EventBeginPlay
  (CallFunction|AddSoundDurations)
  (Audio|PlaySound2D (Utilities|Array|Get(acopy) (Variables|Default|GetPlaylist)) 1.0 1.0 0.0 0 0)
  (Utilities|Time|SetTimerbyEvent (delegate Custom|PlayNextSong) (Utilities|Array|Get(acopy) (Variables|Default|GetSongLengths))))

(fn ConstructionScript)

(fn AddSoundDurations
  (for _array_element (Variables|Default|GetPlaylist)
    (Utilities|Array|Add (Variables|Default|GetSongLengths) (Variables|/Script/Engine.SoundBase|GetDuration _array_element))))